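; BP_Nav is an interactable navigation terminal that shows a level name on a text render and selects the destination level.
; On BeginPlay it looks up the current level, enables sparks on Nav1 and reads the repair state from GI_Space.
; Interacting while broken opens the fix widget, and ConsoleFixed saves the repair to the game instance.
; Otherwise, subject to flag checks, interaction advances the selection or engages autopilot at the next level.
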(event `self.ReceiveBeginPlay`
  (bind _currentlevel (`self.CurrentLevel`))
  (`|ExecutionSequence`
    (:`then_0`
      (bind _returnvalue (`GameplayStatics.GetCurrentLevelName` true))
      (set `self.CurrentLevel` (`KismetStringLibrary.Conv_StringToName` _returnvalue))
      (bind _output_get (set `self.LevelArray` (`|MakeArray` "Level1" "Level2" "Level3" :!type "Name")))
      (bind _output_get_2 (set `self.LevelIndex` (`KismetArrayLibrary.Array_Find` _output_get (`self.CurrentLevel`))))
      (`/Engine/EditorBlueprintResources/StandardMacros.IsValid` null
        (:`Is Valid`
          (set `self.LevelSelected` (`|GetArrayItem` (`self.LevelArray`) _output_get_2))
          (`TextRenderComponent.K2_SetText` (`self.TextRender`) (`KismetTextLibrary.Conv_NameToText` _currentlevel))
          (if (== _currentlevel "Nav1")
            (`ActorComponent.Activate` (`self.P_Sparks`) false)))))
    (:`then_1`
      (bind _asgi_space (cast `/Game/FirstPerson/Blueprints/GI_Space` (`GameplayStatics.GetGameInstance`)))
      (bind _output_get_3 (set `self.As GI Space` _asgi_space))
      (set `self.Fixed` (`/Game/FirstPerson/Blueprints/GI_Space.Fixed_GI` _output_get_3)))))

(event `ConsoleFixed`
  (`ActorComponent.Deactivate` (`self.P_Sparks`))
  (bind _output_get (set `self.Fixed` true))
  (set `/Game/FirstPerson/Blueprints/GI_Space.Fixed_GI` _output_get (`self.As GI Space`)))

(event `/Game/Blueprints/BlueprintInterfaces/IBP_Interact.Interact`
  (if (`self.butlerdrinkspiss`)
    (if (`self.go`)
      (if (== (`self.LevelIndex`) (+ (`KismetArrayLibrary.Array_Find` (`self.LevelArray`) (`self.CurrentLevel`)) 1)) :!label _label
        (set `self.AutoPilotEngaged` true)
        (else
          (bind _result (`/Engine/EditorBlueprintResources/StandardMacros.IncrementInt` (`self.LevelIndex`))
            (:`  `
              (set `self.LevelIndex` _result)
              (bind _output_get (set `self.LevelSelected` (`|GetArrayItem` (`self.LevelArray`) (`self.LevelIndex`))))
              (`TextRenderComponent.K2_SetText` (`self.TextRender`) (`KismetTextLibrary.Conv_NameToText` _output_get)))))))
    (elif (not (`self.Fixed`))
      (bind _returnvalue (`|CreateWidget` "/Game/Blueprints/WorldMechanics/NavSystem/WBP_FixNavTerminal.WBP_FixNavTerminal_C"))
      (`UserWidget.AddToViewport` _returnvalue 0)
      (else
        (goto _label)))))

(fn `UserConstructionScript`)