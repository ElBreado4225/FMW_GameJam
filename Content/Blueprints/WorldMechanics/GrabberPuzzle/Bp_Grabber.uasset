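; Grabber from the grabber puzzle mechanics that throws a grapple hand on a roped cable when the left mouse button is released.
; A camera-forward sphere trace sets the throw direction for a spawned Bp_GrabberHand, linked to the grabber by a Bp_Rope.
; Timelines adjust cable length and trigger retraction beyond GrappleReach.
; Retraction respawns hand and rope, launches the collisionless hand back toward the Swing socket, then destroys both.
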(event `Key|LeftMouseButton`
  (params (Key :type "Key Structure"))
  (bind _followcamera (`self.FollowCamera`))
  (bind _returnvalue (`SceneComponent.K2_GetComponentLocation` _followcamera))
  (bind _returnvalue_location (`KismetMathLibrary.BreakTransform` (`SceneComponent.GetSocketTransform` (`self.HookSkeleton`) "Swing" "RTS_World")))
  (bind _returnvalue_2 (`SceneComponent.K2_GetComponentLocation` (`self.SpawnHook`)))
  ; Grapple
  (:`Released`
    (if true
      ;; Debug For Throw Direction
      (bind (_outhit _returnvalue_3) (`KismetSystemLibrary.SphereTraceSingle` _returnvalue (+ _returnvalue (* (`KismetMathLibrary.GetForwardVector` (`SceneComponent.K2_GetComponentRotation` _followcamera)) (`self.GrappleReach`))) 100.0 "TraceTypeQuery1"))
      (bind (_bblockinghit _binitialoverlap _time _distance _location _impactpoint _normal _impactnormal _physmat _hitactor _hitcomponent _hitbonename _bonename _hititem _elementindex _faceindex _tracestart _traceend) (`GameplayStatics.BreakHitResult` _outhit))
      ;; Target Location On Hit
      (set `self.SwingLocation` (select `bool` _returnvalue_3 :`false` _impactpoint :`true` _traceend))
      ;; Spawn grapple Actor
      (set `self.ThrowDirection` _returnvalue_2)
      (bind _returnvalue_4 (`|SpawnActorFromClass` "/Game/Blueprints/WorldMechanics/GrabberPuzzle/Bp_GrabberHand.Bp_GrabberHand_C" (`KismetMathLibrary.MakeTransform` _returnvalue_2 (`SceneComponent.K2_GetComponentRotation` (`self.FollowCamera`))) "Undefined" "MultiplyWithRoot" null (* (`KismetMathLibrary.Normal` (- (`self.SwingLocation`) _returnvalue_2)) (`self.ThrowSpeed`)) null))
      (bind _output_get (set `self.GrabberHand` _returnvalue_4))
      (`PrimitiveComponent.SetCollisionEnabled` (`/Game/Blueprints/WorldMechanics/GrabberPuzzle/Bp_GrabberHand.GrappleHand` _output_get) "QueryAndPhysics")
      ;; Comment
      (bind _returnvalue_5 (`|SpawnActorFromClass` "/Game/Blueprints/WorldMechanics/GrabberPuzzle/Bp_Rope.Bp_Rope_C" (`KismetMathLibrary.MakeTransform` _returnvalue_location (`KismetMathLibrary.MakeRotFromX` (`self.ThrowDirection`))) "Undefined" "MultiplyWithRoot" null null))
      (bind _output_get_2 (set `self.GrappleRope` _returnvalue_5))
      (`self.K2_AttachToActor` _output_get_2 self "None" "KeepWorld" "KeepWorld" "KeepWorld" true)
      (`CableComponent.SetAttachEndTo` (`CableActor.CableComponent` (`self.GrappleRope`)) (`self.GrabberHand`) "None" "Rope")
      (`self.StartGrappleTimer`)
      (else
        (`self.RetractHook`)))))

(event `RetractHook`
  (bind _grappletransform_location (`KismetMathLibrary.BreakTransform` (`self.GrappleTransform`)))
  (bind (_grappletransform_location_2 _grappletransform_rotation) (`KismetMathLibrary.BreakTransform` (`self.GrappleTransform`)))
  (bind _grappletransform_location_3 (`KismetMathLibrary.BreakTransform` (`self.GrappleTransform`)))
  (bind _returnvalue_location (`KismetMathLibrary.BreakTransform` (`SceneComponent.GetSocketTransform` (`self.HookSkeleton`) "Swing" "RTS_World")))
  (bind _returnvalue_location_2 (`KismetMathLibrary.BreakTransform` (`SceneComponent.GetSocketTransform` (`self.HookSkeleton`) "Swing" "RTS_World")))
  (bind _returnvalue_location_3 (`KismetMathLibrary.BreakTransform` (`SceneComponent.GetSocketTransform` (`self.HookSkeleton`) "Swing" "RTS_World")))
  ; Grapple
  ;; Last Position of Hook
  (set `self.GrappleTransform` (`self.GetTransform` (`self.GrabberHand`)) :!label _label)
  (`/Engine/EditorBlueprintResources/StandardMacros.IsValid` (`self.GrappleRope`)
    (:`Is Valid`
      (`self.K2_DestroyActor` (`self.GrabberHand`))
      (`self.K2_DestroyActor` (`self.GrappleRope`))
      (bind _returnvalue (`|SpawnActorFromClass` "/Game/Blueprints/WorldMechanics/GrabberPuzzle/Bp_GrabberHand.Bp_GrabberHand_C" (`KismetMathLibrary.MakeTransform` _grappletransform_location_2 _grappletransform_rotation) "Undefined" "MultiplyWithRoot" null (* (`KismetMathLibrary.Normal` (- _grappletransform_location_3 _returnvalue_location_3)) (+ (`KismetMathLibrary.Vector_Distance` _returnvalue_location_2 _grappletransform_location) 500.0) -1.0) null))
      (bind _output_get (set `self.GrabberHand` _returnvalue))
      (`PrimitiveComponent.SetCollisionEnabled` (`/Game/Blueprints/WorldMechanics/GrabberPuzzle/Bp_GrabberHand.GrappleHand` _output_get) "NoCollision")
      (bind _returnvalue_2 (`|SpawnActorFromClass` "/Game/Blueprints/WorldMechanics/GrabberPuzzle/Bp_Rope.Bp_Rope_C" (`KismetMathLibrary.MakeTransform` _returnvalue_location (`KismetMathLibrary.MakeRotFromX` (`self.ThrowDirection`))) "Undefined" "MultiplyWithRoot" null null))
      (bind _output_get_2 (set `self.GrappleRope` _returnvalue_2))
      (`self.K2_AttachToActor` _output_get_2 self "None" "KeepWorld" "KeepWorld" "KeepWorld" true)
      (`CableComponent.SetAttachEndTo` (`CableActor.CableComponent` (`self.GrappleRope`)) (`self.GrabberHand`) "None" "Rope")
      ;; Destroy Hook And Reset
      (`self.StopGrappleEvent`)
      (`KismetSystemLibrary.Delay` 0.7)
      (`self.K2_DestroyActor` (`self.GrappleRope`))
      (`self.K2_DestroyActor` (`self.GrabberHand`)))))

(event `StartGrappleTimer`
  (bind _grabberhand (`self.GrabberHand`))
  (bind _returnvalue_location (`KismetMathLibrary.BreakTransform` (`SceneComponent.GetSocketTransform` (`self.HookSkeleton`) "Swing" "RTS_World")))
  (bind _cablecomponent (`CableActor.CableComponent` (`self.GrappleRope`)))
  ; Grapple
  (`|ExecutionSequence`
    (:`then_0`
      (`Timeline|Timeline` :!label _label_2
        (:`Update`
          (if (> (`KismetMathLibrary.Vector_Distance` (`/Game/Blueprints/WorldMechanics/GrabberPuzzle/Bp_GrabberHand.StartLocation` _grabberhand) (`self.K2_GetActorLocation` _grabberhand)) (`self.GrappleReach`))
            (goto _label)))))
    (:`then_1`
      ;; UpdateCableLength
      (`KismetSystemLibrary.Delay` 0.5)
      (`Timeline|Timeline_0` :!label _label_3
        (:`Update`
          (`/Engine/EditorBlueprintResources/StandardMacros.IsValid` _cablecomponent
            (:`Is Valid`
              (set `CableComponent.CableLength` (`KismetMathLibrary.FClamp` (- (`KismetMathLibrary.Vector_Distance` _returnvalue_location (`SceneComponent.K2_GetComponentLocation` (`/Game/Blueprints/WorldMechanics/GrabberPuzzle/Bp_GrabberHand.GrappleHand` (`self.GrabberHand`)))) 150.0) 150.0 1000.0) _cablecomponent))))))))

(event `StopGrappleEvent`
  ; Grapple
  (`|ExecutionSequence`
    (:`then_0`
      (goto _label_2 :!via `Stop`))
    (:`then_1`
      (goto _label_3 :!via `Stop`))))

(fn `UserConstructionScript`)