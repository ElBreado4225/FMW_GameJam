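; Projectile grappling hand for the grabber puzzle that launches on spawn and changes course when it touches something.
; BeginPlay caches the first-person player, applies its Velocity variable to ProjectileMovement and stores a hardcoded start location.
; Box overlap sets a hit flag, records and prints the hand's location as the hooked point, then plays a timeline that forces a fixed, mostly +X velocity on every update.
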(event `self.ReceiveBeginPlay`
  (bind _asbp_first_person_character (cast `/Game/FirstPerson/Blueprints/BP_FirstPersonCharacter` (`GameplayStatics.GetPlayerPawn` 0)))
  (set `self.As BP First Person Character` _asbp_first_person_character)
  (set `MovementComponent.Velocity` (`self.Velocity`) (`self.ProjectileMovement`))
  (set `self.StartLocation` (1640.0 -1220.0 -1220.0)))

(event `self.Box.OnComponentBeginOverlap`
  (params (OverlappedComponent :type "PrimitiveComponent Object Reference") (OtherActor :type "Actor Object Reference") (OtherComp :type "PrimitiveComponent Object Reference") (OtherBodyIndex :type Integer) (bFromSweep :type Boolean) (SweepResult :type "HitResult Structure (by ref)"))
  (set `self.Hit?` true)
  (bind _output_get (set `self.HookedLocation` (`SceneComponent.K2_GetComponentLocation` (`self.GrappleHand`))))
  (`KismetSystemLibrary.PrintString` (`KismetStringLibrary.Conv_VectorToString` _output_get))
  (`Timeline|Timeline`
    (:`Update`
      (set `MovementComponent.Velocity` (380.0 0.0 -5.0) (`self.ProjectileMovement`)))))

(fn `UserConstructionScript`)