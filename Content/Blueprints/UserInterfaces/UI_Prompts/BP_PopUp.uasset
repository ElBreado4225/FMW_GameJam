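; BP_PopUp is a trigger that shows a text prompt on screen when something begins overlapping its Box component.
; Each overlap creates a WBP_FirstWakeUpPrompt, adds it to the viewport, then sets its text from FullText after a short delay.
; After Duration elapses it plays the widget's DropDown animation in reverse.
; The graph has no actor filter or once-only guard, and never removes the widget.
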(event `self.Box.OnComponentBeginOverlap`
  (params (OverlappedComponent :type "PrimitiveComponent Object Reference") (OtherActor :type "Actor Object Reference") (OtherComp :type "PrimitiveComponent Object Reference") (OtherBodyIndex :type Integer) (bFromSweep :type Boolean) (SweepResult :type "HitResult Structure (by ref)"))
  (bind _widgetref (`self.WidgetRef`))
  (bind _returnvalue (`|CreateWidget` "/Game/Blueprints/UserInterfaces/UI_Prompts/WBP_FirstWakeUpPrompt.WBP_FirstWakeUpPrompt_C"))
  (bind _output_get (set `self.WidgetRef` _returnvalue))
  (`UserWidget.AddToViewport` _output_get 0)
  (`KismetSystemLibrary.Delay` 0.5)
  (`/Game/Blueprints/UserInterfaces/UI_Prompts/WBP_FirstWakeUpPrompt.UpdateText` _widgetref (`self.Full Text`))
  (`KismetSystemLibrary.Delay` (`self.Duration`))
  (`UserWidget.PlayAnimation` _widgetref (`/Game/Blueprints/UserInterfaces/UI_Prompts/WBP_FirstWakeUpPrompt.DropDown` _widgetref) 0.0 1 "Reverse" 1.0 false))

(fn `UserConstructionScript`)